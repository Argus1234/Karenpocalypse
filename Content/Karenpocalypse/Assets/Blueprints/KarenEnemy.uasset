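; KarenEnemy is an enemy that chases the player and deals punch damage at close range.
; Every Tick it issues an AI MoveTo toward the FirstPersonCharacter, then immediately checks whether the player overlaps its AttackSphere.
; While overlapping, PunchDamage subtracts PunchDamageAmount directly from the player's integer PlayerHealth, truncating the result.
; The damage has no cooldown, so it repeats every frame.
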(event EventBeginPlay)

(event Collision|EventActorBeginOverlap
  (params (OtherActor :type Actor%20Object%20Reference)))

(event EventTick
  (params (DeltaSeconds :type Float%20%28single-precision%29))
  (bind _asfirst_person_character (Utilities|Casting|CastToFirstPersonCharacter (Game|GetPlayerCharacter 0)))
  (AI|AIMoveTo self "0, 0, 0" _asfirst_person_character 5.0 false
    (:then
      (bind _asfirst_person_character_2 (Utilities|Casting|CastToFirstPersonCharacter (Game|GetPlayerCharacter 0)))
      (if (Utilities|Array|ContainsItem (Collision|GetOverlappingActors (Variables|Default|GetAttackSphere) "/Game/FirstPersonBP/Blueprints/FirstPersonCharacter.FirstPersonCharacter_C" :!class /Script/Engine.PrimitiveComponent) _asfirst_person_character_2)
        (CallFunction|PunchDamage)))))

(fn ConstructionScript)

(fn PunchDamage
  (bind _asfirst_person_character (Utilities|Casting|CastToFirstPersonCharacter (Game|GetPlayerCharacter 0)))
  (Variables|/Game/FirstPersonBP/Blueprints/FirstPersonCharacter.FirstPersonCharacter_C|SetPlayerHealth _asfirst_person_character (Math|Float|Truncate (- (Math|Conversions|ToFloat(Integer) (Variables|/Game/FirstPersonBP/Blueprints/FirstPersonCharacter.FirstPersonCharacter_C|GetPlayerHealth _asfirst_person_character)) (Variables|Default|GetPunchDamageAmount)))))